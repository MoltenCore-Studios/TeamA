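; Forging station Blueprint that animates a hammer swing at one of three target hit points, chosen by index.
; PlayHammerAnimation moves the hammer pivot to the chosen target's X, then computes a look-at rotation toward it and a second rotation offset by a 90-degree pitch.
; The HammerSwingTL timeline lerps the pivot between those rotations along the shortest path.
; Visual_StrikeAtLocation is an empty event.
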(event `Visual_StrikeAtLocation`
  (params (TargetLocation :type "Vector Structure")))

(event `self.PlayHammerAnimation`
  (params (HammerIndex :type Integer) (Quality :type "EForgeHitQuality Enum" :default "Perfect"))
  (bind _returnvalue (select `int` HammerIndex :`0` (`SceneComponent.K2_GetComponentLocation` (`self.TARGET_HIT_0`)) :`1` (`SceneComponent.K2_GetComponentLocation` (`self.TARGET_HIT_1`)) :`2` (`SceneComponent.K2_GetComponentLocation` (`self.TARGET_HIT_2`))))
  (bind _returnvalue_2 (`KismetMathLibrary.MakeVector` (.x _returnvalue) (.y (`SceneComponent.K2_GetComponentLocation` (`self.HammerPivot`))) (.z (`SceneComponent.K2_GetComponentLocation` (`self.HammerPivot`)))))
  (bind _returnvalue_3 (`KismetMathLibrary.FindLookAtRotation` _returnvalue_2 _returnvalue))
  (`SceneComponent.K2_SetWorldLocation` (`self.HammerPivot`) _returnvalue_2 false true)
  (set `self.StartRotation` _returnvalue_3)
  (set `self.EndRotation` (`KismetMathLibrary.ComposeRotators` _returnvalue_3 (struct :`Roll` 90.0)))
  (bind (_direction _alpha) (`Timeline|HammerSwingTL` :!via `PlayFromStart`)
    (:`Update`
      (`SceneComponent.K2_SetWorldRotation` (`self.HammerPivot`) (`KismetMathLibrary.RLerp` (`self.StartRotation`) (`self.EndRotation`) _alpha true) false false))))

(fn `UserConstructionScript`)