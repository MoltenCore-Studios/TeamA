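; Workstation actor where a player manipulates the first inventory item with the mouse and keys while a component spins.
; Enter and Exit toggle input, cursor and a Tick gate that moves the item to the cursor hit point near an arrow, returning it to its slot on close.
; Move input rotates the item.
; Space adds clamped spin to Spinny, whose timeline replays recursively as the value decays.
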(event `self.Exit`
  (params (Character :type "Character Object Reference"))
  (bind _returnvalue (`GameplayStatics.GetPlayerController` 0))
  (`self.DisableInput` _returnvalue)
  (set `PlayerController.bShowMouseCursor` false _returnvalue)
  (`self.CloseGate`))

(event `self.Enter`
  (params (Character :type "Character Object Reference"))
  (bind _returnvalue (`GameplayStatics.GetPlayerController` 0))
  (set `self.Character` Character)
  (`KismetSystemLibrary.PrintString` (`KismetSystemLibrary.GetDisplayName` (`|GetArrayItem` (`self.Inventory`))))
  (`self.EnableInput` _returnvalue)
  (set `PlayerController.bShowMouseCursor` true _returnvalue)
  (`self.OpenGate`))

(event `ContinueSpin`
  (bind _wheelrot (`self.WheelRot`))
  (set `self.WheelRot` (`SceneComponent.K2_GetComponentRotation` (`self.Spinny`)) :!label _label)
  (bind (_direction _alpha) (`Timeline|Timeline` :!via `PlayFromStart`)
    (:`Update`
      (`SceneComponent.K2_SetWorldRotation` (`self.Spinny`) (`KismetMathLibrary.RLerp` _wheelrot (`KismetMathLibrary.MakeRotator` (+ (.roll _wheelrot) (`self.SpinValue`)) (.pitch _wheelrot) (.yaw _wheelrot)) _alpha true) false false))
    (:`Finished`
      (if (> (`self.SpinValue`) 0.0)
        (set `self.SpinValue` (`KismetMathLibrary.FClamp` (- (`self.SpinValue`) 10.0) 0.0 170.0))
        (`self.ContinueSpin`)))))

(event `EnhancedInput|/Game/Input/Actions/IA_Space`
  (params (ActionValue :type Boolean) (ElapsedSeconds :type "Float (double-precision)") (TriggeredSeconds :type "Float (double-precision)") (InputAction :type "InputAction Object Reference" :default "/Game/Input/Actions/IA_Space.IA_Space"))
  (:`Started`
    (`KismetSystemLibrary.PrintString` "Hello")
    (set `self.SpinValue` (`KismetMathLibrary.FClamp` (+ (`self.SpinValue`) 10.0) 0.0 170.0))
    (goto _label)))

(event `EnhancedInput|/Game/Input/Actions/IA_Move`
  (params (ActionValue :type "Vector2D Structure") (ElapsedSeconds :type "Float (double-precision)") (TriggeredSeconds :type "Float (double-precision)") (InputAction :type "InputAction Object Reference" :default "/Game/Input/Actions/IA_Move.IA_Move"))
  (bind (_x _y) (`KismetMathLibrary.BreakVector2D` ActionValue))
  (:`Triggered`
    (`self.RotateProject` false _y)
    (`self.RotateProject` true _x)))

(event `self.ReceiveTick`
  (params (DeltaSeconds :type "Float (single-precision)"))
  (bind (_hitresult _returnvalue) (`PlayerController.GetHitResultUnderCursorByChannel` (`GameplayStatics.GetPlayerController` 0) "TraceTypeQuery1" true))
  (bind _output (`|GetArrayItem` (`self.Inventory`)))
  (`/Engine/EditorBlueprintResources/StandardMacros.Gate` true :!label _label_2
    (:`Exit`
      (`/Engine/EditorBlueprintResources/StandardMacros.IsValid` _output
        (:`Is Valid`
          (if _returnvalue
            (if (not (> (`KismetMathLibrary.Vector_Distance` (`.Location` (`GameplayStatics.BreakHitResult` _hitresult)) (`SceneComponent.K2_GetComponentLocation` (`self.Arrow`))) 400.0))
              (`SceneComponent.K2_SetWorldLocation` (`Pickup.CollisionMesh` _output) (`.Location` (`GameplayStatics.BreakHitResult` _hitresult)) false false))))))))

(event `OpenGate`
  (goto _label_2 :!via `Open`))

(event `CloseGate`
  (`|ExecutionSequence`
    (:`then_0`
      (goto _label_2 :!via `Close`))
    (:`then_1`
      (`KismetSystemLibrary.Delay` 0.01)
      (`SceneComponent.K2_SetWorldLocation` (`Pickup.CollisionMesh` (`|GetArrayItem` (`self.Inventory`))) (`SceneComponent.K2_GetComponentLocation` (`self.ItemSlot`)) false false))))

(fn `LowerSpinValue`
  (params (Alpha :type "Float (double-precision)")))

(fn `RotateProject`
  (params (`X?` :type Boolean) (Value :type "Float (double-precision)"))
  (bind _returnvalue (* 2.0 Value))
  (bind _output (`|GetArrayItem` (`self.Inventory`)))
  (`/Engine/EditorBlueprintResources/StandardMacros.IsValid` _output
    (:`Is Valid`
      (if `X?`
        (`self.K2_AddActorWorldRotation` _output (`KismetMathLibrary.MakeRotator` (* _returnvalue -1.0)) false false)
        (else
          (`self.K2_AddActorWorldRotation` _output (`KismetMathLibrary.MakeRotator` 0.0 _returnvalue) false false))))))

(fn `UserConstructionScript`)