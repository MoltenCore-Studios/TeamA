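; Workstation Blueprint that triggers the assembly minigame based on the contents of its Inventory.
; Enter starts the first BP_AssemblyMinigame found in the level when the Inventory holds exactly one item, an index check that assumes single-item placement.
; Exit calls RestartMinigame on that actor unless the Inventory is empty, in which case it only prints a debug message.
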(event `self.ReceiveActorBeginOverlap`
  (params (OtherActor :type "Actor Object Reference")))

(event `self.Enter`
  (params (Character :type "Character Object Reference"))
  (bind _returnvalue (`KismetArrayLibrary.Array_LastIndex` (`self.Inventory`)))
  ; Please Note, this only works if only one item can be place on they, if it can't please re-evaluate the index so the conditions are correct
  (`KismetSystemLibrary.PrintString` (`KismetStringLibrary.Conv_IntToString` _returnvalue))
  (if (== _returnvalue 0)
    (bind _outactors (`GameplayStatics.GetAllActorsOfClass` "/Game/Tyrell_folder/BP_AssemblyMinigame.BP_AssemblyMinigame_C"))
    (`/Game/Tyrell_folder/BP_AssemblyMinigame.StartMinigame()` (`|GetArrayItem` _outactors))))

(event `self.Exit`
  (params (Character :type "Character Object Reference"))
  ; Please Note, this only works if only one item can be place on they, if it can't please re-evaluate the index so the conditions are correct
  (if (== (`KismetArrayLibrary.Array_LastIndex` (`self.Inventory`)) -1)
    (`KismetSystemLibrary.PrintString` "they are no items")
    (else
      (bind _outactors (`GameplayStatics.GetAllActorsOfClass` "/Game/Tyrell_folder/BP_AssemblyMinigame.BP_AssemblyMinigame_C"))
      (`/Game/Tyrell_folder/BP_AssemblyMinigame.Restart_minigame` (`|GetArrayItem` _outactors)))))

(fn `UserConstructionScript`)