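; Job manager for a weapon-crafting notice board, generating random orders and handling the player's response to them.
; On BeginPlay it builds jobs from weapon and metal data tables, spawning BP_Task posters at trace-checked free board points.
; Picking one up pauses the game and shows its WB_Poster; accepting moves it to a free WeaponHolder.
; Taken jobs can be sold or scrapped, though payment is a stub and EE jobs are switched off.
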(event `self.ReceiveBeginPlay`
  ; Begin Play
  (bind _outactors (`GameplayStatics.GetAllActorsOfClass` "/Game/Connor_Folder/NoticeBoard/JobCompletion/WeaponHolder.WeaponHolder_C"))
  (set `self.Weapon Holders` _outactors)
  (`self.Grab Key Components`)
  (for _ (range 1 (+ (`self.Number of Jobs`) 1))
    (`self.Create a job`)))

(event `Grab Key Components`
  ; Grabbing the data it needs to create jobs
  (bind _outrownames (`DataTableFunctionLibrary.GetDataTableRowNames` "/Game/Connor_Folder/NoticeBoard/DT_Weapons.DT_Weapons"))
  (set `self.Weapons` _outrownames)
  (bind _outrownames_2 (`DataTableFunctionLibrary.GetDataTableRowNames` "/Game/Connor_Folder/NoticeBoard/DT_Metals.DT_Metals"))
  (set `self.Metals` _outrownames_2)
  (bind _outrownames_3 (`DataTableFunctionLibrary.GetDataTableRowNames` "/Game/Connor_Folder/NoticeBoard/DT_EEJobs.DT_EEJobs"))
  (set `self.EE jobs` _outrownames_3)
  (bind _returnvalue (`GameplayStatics.GetActorOfClass` "/Game/Connor_Folder/NoticeBoard/NoticeBoard.NoticeBoard_C"))
  (set `self.NoticeBoard` _returnvalue))

(event `Create a job`
  ; Creating the jobs and adding key information to arrays
  (bind (_weapon_name _metal_name _description _expected_payout) (`self.CreateJob` false))
  (`KismetArrayLibrary.Array_Add` (`self.Jobs`) (make `/Game/Connor_Folder/NoticeBoard/Job_Struct` _weapon_name _metal_name _expected_payout))
  (bind _returnvalue (`|CreateWidget` "/Game/Connor_Folder/NoticeBoard/WB_Poster.WB_Poster_C" null _description))
  (`KismetArrayLibrary.Array_Add` (`self.JobWidgets`) _returnvalue)
  (bind (_canspawn _location _rotation) (`self.GetPosterSpawnPoint`))
  (if _canspawn
    (bind _returnvalue_2 (`|SpawnActorFromClass` "/Game/Connor_Folder/NoticeBoard/BP_Task.BP_Task_C" (`KismetMathLibrary.MakeTransform` _location _rotation) "AlwaysSpawn" "MultiplyWithRoot" null self _description false null))
    (`KismetArrayLibrary.Array_Add` (`self.JobPosters`) _returnvalue_2)
    (else
      (`KismetSystemLibrary.PrintString` "Job Board Full"))))

(event `PickUpPoster`
  (params (Caller :type "/Game/Connor_Folder/NoticeBoard/BP_Task Object Reference") (TakenJob :type Boolean))
  (bind _output (`|GetArrayItem` (`self.JobWidgets`) (`KismetArrayLibrary.Array_Find` (`self.JobPosters`) Caller)))
  (bind _output_2 (`|GetArrayItem` (`self.JobWidgets`) (`KismetArrayLibrary.Array_Find` (`self.JobPosters`) Caller)))
  ; Called from the BP_Task actor, gets which job the player selected
  (set `self.Taken Job` TakenJob)
  (`/Engine/EditorBlueprintResources/StandardMacros.DoOnce` false :!label _label
    (:`Completed`
      (if (not (`self.Taken Job`))
        (bind (_return _index) (`self.MoveJobToSpot`))
        (set `self.HolderIndex` _index)
        (if _return
          (`UserWidget.AddToViewport` _output_2 0)
          (`/Game/Connor_Folder/NoticeBoard/WB_Poster.Grabbed` _output_2)
          (`self.SetActorHiddenInGame` Caller true)
          (`GameplayStatics.SetGamePaused` true)
          (else
            (set `/Game/Connor_Folder/NoticeBoard/BP_Task.Taken` false Caller :!label _label_2)
            (goto _label :!via `Reset`)))
        (else
          (`KismetSystemLibrary.PrintString` "TakenJob")
          (`UserWidget.AddToViewport` _output 0)
          (`/Game/Connor_Folder/NoticeBoard/WB_Poster.Grabbed` _output)
          (`self.SetActorHiddenInGame` Caller true)
          (`GameplayStatics.SetGamePaused` true))))))

(event `/Game/Connor_Folder/NoticeBoard/BPI_SpeakToManager.PosterRespond`
  (params (Response :type String) (Who :type "/Game/Connor_Folder/NoticeBoard/WB_Poster Object Reference"))
  (bind _jobwidgets (`self.JobWidgets`))
  (bind _jobs (`self.Jobs`))
  (bind _jobposters (`self.JobPosters`))
  (bind _returnvalue (`KismetArrayLibrary.Array_Find` _jobwidgets Who))
  (bind _output (`|GetArrayItem` (`self.Weapon Holders`) (`self.HolderIndex`)))
  (bind _output_2 (`|GetArrayItem` _jobposters _returnvalue))
  (bind _output_3 (`|GetArrayItem` (`self.JobPosters`) _returnvalue))
  (bind (_returnvalue_location _returnvalue_rotation) (`KismetMathLibrary.BreakTransform` (`SceneComponent.K2_GetComponentToWorld` (`/Game/Connor_Folder/NoticeBoard/JobCompletion/WeaponHolder.PosterSpot` (`|GetArrayItem` (`self.Weapon Holders`) (`self.HolderIndex`))))))
  (`GameplayStatics.SetGamePaused` false)
  (if (not (`self.Taken Job`))
    (switch `string` Response
      (:`Accept`
        (set `/Game/Connor_Folder/NoticeBoard/JobCompletion/WeaponHolder.RelatedJob` (`|GetArrayItem` (`self.Jobs`) _returnvalue) _output)
        (set `/Game/Connor_Folder/NoticeBoard/BP_Task.RelatedHolder` _output _output_3)
        (`self.K2_SetActorTransform` _output_3 (`KismetMathLibrary.MakeTransform` _returnvalue_location _returnvalue_rotation) false false)
        (`self.SetActorHiddenInGame` _output_3 false)
        (goto _label :!via `Reset`))
      (:`DecideLater`
        (`self.SetActorHiddenInGame` _output_3 false))
      (:`Decline`
        (`KismetArrayLibrary.Array_RemoveItem` _jobs (`|GetArrayItem` _jobs _returnvalue))
        (`self.K2_DestroyActor` _output_2)
        (`KismetArrayLibrary.Array_RemoveItem` _jobposters _output_2)
        (`KismetArrayLibrary.Array_RemoveItem` _jobwidgets Who)))
    ; Called from the BP_Task actor, gets which job the player selected
    (set `/Game/Connor_Folder/NoticeBoard/JobCompletion/WeaponHolder.Taken` false (`|GetArrayItem` (`self.Weapon Holders`) (`self.HolderIndex`)))
    (goto _label_2)
    (else
      (switch `string` Response
        (:`Accept`
          (`KismetSystemLibrary.PrintString` "Sold")
          (`self.Sell`))
        (:`DecideLater`
          (`KismetSystemLibrary.PrintString` "DecideLater")
          (`self.SetActorHiddenInGame` (`|GetArrayItem` (`self.JobPosters`) (`KismetArrayLibrary.Array_Find` (`self.JobWidgets`) Who)) false)
          (goto _label :!via `Reset`))
        (:`Decline`
          (`KismetSystemLibrary.PrintString` "Scrapped")
          (`self.Scrap`))))))

(event `Sell`
  (bind _jobs (`self.Jobs`))
  (`KismetSystemLibrary.PrintString` "Code here that rates and gives money")
  (bind _returnvalue (`KismetArrayLibrary.Array_Find` (`self.JobWidgets`) (stale `/Game/Connor_Folder/NoticeBoard/BPI_SpeakToManager.PosterRespond` Who)))
  (`KismetArrayLibrary.Array_RemoveItem` _jobs (`|GetArrayItem` _jobs _returnvalue) :!label _label_3)
  (bind _output (`|GetArrayItem` (`self.JobPosters`) _returnvalue))
  (set `/Game/Connor_Folder/NoticeBoard/JobCompletion/WeaponHolder.Taken` false (`/Game/Connor_Folder/NoticeBoard/BP_Task.RelatedHolder` _output))
  (`self.K2_DestroyActor` _output)
  (`KismetArrayLibrary.Array_RemoveItem` (`self.JobPosters`) _output)
  (`KismetArrayLibrary.Array_RemoveItem` (`self.JobWidgets`) (stale `/Game/Connor_Folder/NoticeBoard/BPI_SpeakToManager.PosterRespond` Who))
  (goto _label :!via `Reset`))

(event `Scrap`
  (goto _label_3))

(fn `CreateJob`
  (params (IncludeEE :type Boolean))
  (returns (`Weapon name` :type String) (`Metal Name` :type String) (Description :type String) (`Expected Payout` :type "Float (double-precision)"))
  (locals (`Selected Weapon from DT` :type Name) (`Selected Metal from DT` :type Name) (WeaponStruct :type "/Game/Connor_Folder/NoticeBoard/WeaponType_Struct Structure") (MetalStruct :type "/Game/Connor_Folder/NoticeBoard/MetalType_Struct Structure") (`Select EE from DT` :type Name) (EEStruct :type "/Game/Connor_Folder/NoticeBoard/EasterEggJobs Structure"))
  ; getting the information needed to create a job from data tables
  (if (and IncludeEE (== (`KismetMathLibrary.RandomIntegerInRange` 1 10) 1))
    (set `local.Select EE from DT` (`KismetArrayLibrary.Array_Random` (`self.EE jobs`)))
    (bind _returnvalue (`|GetDataTableRow` "/Game/Connor_Folder/NoticeBoard/DT_EEJobs.DT_EEJobs" (`local.Select EE from DT`))
      (:`then`
        (bind _output_get (set `local.EEStruct` _returnvalue))
        (bind (_description _weapon _metal _price) (`self.EEJobBreakdown` _output_get))
        (return _weapon _metal _description _price)))
    (else
      (set `local.Selected Weapon from DT` (`KismetArrayLibrary.Array_Random` (`self.Weapons`)))
      (set `local.Selected Metal from DT` (`KismetArrayLibrary.Array_Random` (`self.Metals`)))
      (bind _returnvalue_2 (`|GetDataTableRow` "/Game/Connor_Folder/NoticeBoard/DT_Weapons.DT_Weapons" (`local.Selected Weapon from DT`))
        (:`then`
          (set `local.WeaponStruct` _returnvalue_2)
          (bind _returnvalue_3 (`|GetDataTableRow` "/Game/Connor_Folder/NoticeBoard/DT_Metals.DT_Metals" (`local.Selected Metal from DT`))
            (:`then`
              (set `local.MetalStruct` _returnvalue_3)
              (bind (_weaponname _metalname _description_2 _expectedpayout) (`self.JobStructBreakdown` (`local.WeaponStruct`) (`local.MetalStruct`)))
              (return _weaponname _metalname _description_2 _expectedpayout))))))))

(fn `DescriptionMaker`
  (params (WeaponDescription :type String) (MetalDescription :type String))
  (returns (MadeDescription :type String))
  (locals (Require :type "Array of String") (Made :type "Array of String"))
  ; Creating a description to make each requesti Unique
  (return (`KismetStringLibrary.Concat_StrStr` (`KismetArrayLibrary.Array_Random` (`local.Require`)) WeaponDescription " " (`KismetArrayLibrary.Array_Random` (`local.Made`)) MetalDescription)))

(fn `EEJobBreakdown`
  (params (EE :type "/Game/Connor_Folder/NoticeBoard/EasterEggJobs Structure"))
  (returns (Description :type String) (Weapon :type String) (Metal :type String) (Price :type "Float (double-precision)"))
  (bind (_name _description _metals _weapons) (break `/Game/Connor_Folder/NoticeBoard/EasterEggJobs` EE))
  (return (`KismetStringLibrary.Concat_StrStr` (`KismetStringLibrary.Concat_StrStr` "From " _name " \n" _description) " \n___________ \n" (`KismetStringLibrary.Concat_StrStr` "I need a " _weapons " made of " _metals)) _weapons _metals 0.0))

(fn `GetPosterSpawnPoint`
  (returns (CanSpawn :type Boolean) (Location :type "Vector Structure") (Rotation :type "Rotator Structure"))
  (locals (CurrentSelectedPoint :type "SceneComponent Object Reference") (`All Points` :type "Array of SceneComponent Object Reference"))
  (bind _currentselectedpoint (`local.CurrentSelectedPoint`))
  ; checking the notice board to see if there is a free spot for a poster to spawn
  (bind _output_get (set `local.All Points` (`SceneComponent.GetChildrenComponents` (`/Game/Connor_Folder/NoticeBoard/NoticeBoard.PosterPoints` (`self.NoticeBoard`)) false)))
  (if (`KismetArrayLibrary.Array_IsNotEmpty` _output_get) :!label _label
    (bind _output_get_2 (set `local.CurrentSelectedPoint` (`KismetArrayLibrary.Array_Random` _output_get)))
    (bind _returnvalue (`SceneComponent.K2_GetComponentLocation` _output_get_2))
    (bind _outhit (`KismetSystemLibrary.SphereTraceSingle` _returnvalue _returnvalue 1.0 "TraceTypeQuery3"))
    (if (or (`GameplayStatics.BreakHitResult` _outhit) (`.bInitialOverlap` (`GameplayStatics.BreakHitResult` _outhit)))
      (`KismetArrayLibrary.Array_RemoveItem` (`local.All Points`) (`local.CurrentSelectedPoint`))
      (goto _label)
      (else
        (return true (`SceneComponent.K2_GetComponentLocation` _currentselectedpoint) (`SceneComponent.K2_GetComponentRotation` _currentselectedpoint))))
    (else
      (return false (0.0 0.0 0.0)))))

(fn `JobStructBreakdown`
  (params (Weapon :type "/Game/Connor_Folder/NoticeBoard/WeaponType_Struct Structure") (Metal :type "/Game/Connor_Folder/NoticeBoard/MetalType_Struct Structure"))
  (returns (WeaponName :type String) (MetalName :type String) (Description :type String) (ExpectedPayout :type "Float (double-precision)"))
  (bind (_metalname _descriptions _metalmesh _ingotvalue) (break `/Game/Connor_Folder/NoticeBoard/MetalType_Struct` Metal))
  (bind (_weaponname _descriptions_2 _ingotcost _weaponactor _basevalue) (break `/Game/Connor_Folder/NoticeBoard/WeaponType_Struct` Weapon))
  ; Grabbing key information from the structs and returning it to the job creation fuction
  (return _weaponname _metalname (`self.DescriptionMaker` (`KismetArrayLibrary.Array_Random` _descriptions_2) (`KismetArrayLibrary.Array_Random` _descriptions)) (+ _basevalue (* _ingotcost _ingotvalue))))

(fn `MoveJobToSpot`
  (returns (Return :type Boolean) (Index :type Integer))
  (locals (IsTaken :type Boolean) (Integer :type Integer))
  (bind _istaken (`local.IsTaken`))
  (set `local.IsTaken` false)
  (for (_array_element _array_index) (`self.Weapon Holders`)
    (if (`/Game/Connor_Folder/NoticeBoard/JobCompletion/WeaponHolder.Taken` _array_element)
      (`KismetSystemLibrary.PrintString` "NO MORE LOCATION")
      (else
        (set `/Game/Connor_Folder/NoticeBoard/JobCompletion/WeaponHolder.Taken` true _array_element)
        (set `local.IsTaken` true)
        (break))))
  (if (not _istaken)
    (`KismetSystemLibrary.PrintString` "None Available"))
  (return _istaken _array_index))

(fn `UserConstructionScript`)