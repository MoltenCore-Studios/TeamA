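; BP_InventoryManager is an inventory Blueprint that holds owned ores in the OresOwned map and handles deductions by metal name.
; Its TakeOutX event subtracts X and writes the result back under that name, printing the name, old value and new value, with no bounds check.
; The old value comes from indexing the map's Values array with the Find result, rather than using that result directly.
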(event `/Game/Connor_Folder/PickUp/Ore/BPI_InventoryManager.TakeOutX`
  (params (X :type Integer) (MetalName :type String))
  (bind _oresowned (`self.OresOwned`))
  (bind _values (`BlueprintMapLibrary.Map_Values` _oresowned))
  (`KismetSystemLibrary.PrintString` MetalName)
  (bind _output (`|GetArrayItem` _values (`BlueprintMapLibrary.Map_Find` _oresowned MetalName)))
  (`KismetSystemLibrary.PrintString` (`KismetStringLibrary.Conv_IntToString` _output))
  (bind _returnvalue (- _output X))
  (`KismetSystemLibrary.PrintString` (`KismetStringLibrary.Conv_IntToString` _returnvalue))
  (`BlueprintMapLibrary.Map_Add` _oresowned MetalName _returnvalue))

(fn `UserConstructionScript`)