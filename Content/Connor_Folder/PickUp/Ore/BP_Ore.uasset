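; BP_Ore is an ore pickup actor whose appearance depends on its Ore value.
; On BeginPlay it looks up that value in DT_Metals and applies the row's mesh and material to its root collision cube.
; PickUp always returns true, while OreBox? reports that it is not an ore box and SpawnOre is an empty stub.
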(event `self.ReceiveBeginPlay`
  (bind _collisioncube_uselikeroot_ (`self.CollisionCube(UseLikeRoot)`))
  (bind _returnvalue (`|GetDataTableRow` "/Game/Connor_Folder/NoticeBoard/DT_Metals.DT_Metals" (`KismetStringLibrary.Conv_StringToName` (`self.Ore`)))
    (:`then`
      (bind _output_get (set `self.MetalInfo` _returnvalue))
      (bind (_metalname _descriptions _metalmesh _ingotvalue _metalmaterial) (break `/Game/Connor_Folder/NoticeBoard/MetalType_Struct` _output_get))
      (`StaticMeshComponent.SetStaticMesh` _collisioncube_uselikeroot_ _metalmesh)
      (`PrimitiveComponent.SetMaterial` _collisioncube_uselikeroot_ 0 _metalmaterial))))

(fn `OreBox?`
  (returns (IsItOreBox :type Boolean) (WhatOre :type String) (IsThereAnOreAvailable :type Boolean) (SpawnPoint :type "Vector Structure"))
  (return false "" false (0.0 0.0 0.0)))

(fn `PickUp`
  (returns (`Can I be Grabbed?` :type Boolean))
  (return true))

(fn `SpawnOre`
  (params (Ore :type String) (Location :type "Vector Structure"))
  (returns (BP_Ore :type "/Game/Connor_Folder/PickUp/Ore/BP_Ore Object Reference"))
  (return null))

(fn `UserConstructionScript`)