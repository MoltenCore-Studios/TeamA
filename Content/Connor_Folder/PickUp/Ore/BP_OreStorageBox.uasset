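; BP_OreStorageBox is a storage box for one ore type, set by WhatBoxIsIt, that dispenses ore from the InventoryManager's owned stock.
; OreBox? reports the ore name, availability and SpawnPoint location, and also removes one unit through TakeOutXMessage whenever its count is positive.
; That count comes from indexing the OresOwned values array with the value Find returns for the ore name.
; PickUp always returns false.
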(event `self.ReceiveBeginPlay`)

(fn `OreBox?`
  (returns (IsItOreBox :type Boolean) (WhatOre :type String) (IsThereAnOreAvailable :type Boolean) (SpawnPoint :type "Vector Structure"))
  (locals (CurrentInBox :type Integer))
  (bind _returnvalue (`|GetEnumeratorNameAsString` (`self.WhatBoxIsIt?`)))
  (bind _returnvalue_2 (> (`local.CurrentInBox`) 0))
  (bind _oresowned (`/Game/Connor_Folder/PickUp/BP_InventoryManager.OresOwned` (`self.InventoryManager`)))
  (bind _values (`BlueprintMapLibrary.Map_Values` _oresowned))
  (set `local.CurrentInBox` (`|GetArrayItem` _values (`BlueprintMapLibrary.Map_Find` _oresowned _returnvalue)))
  (if _returnvalue_2
    (message `/Game/Connor_Folder/PickUp/Ore/BPI_InventoryManager.TakeOutX` (`self.InventoryManager`) 1 _returnvalue))
  (return true _returnvalue _returnvalue_2 (`SceneComponent.K2_GetComponentLocation` (`self.SpawnPoint`))))

(fn `PickUp`
  (returns (`Can I be Grabbed?` :type Boolean))
  (return false))

(fn `UserConstructionScript`)