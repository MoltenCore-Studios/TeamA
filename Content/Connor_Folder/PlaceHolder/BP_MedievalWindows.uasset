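; BP_MedievalWindows is a placeholder window actor that lights up at night and goes dark during the day.
; On BeginPlay it finds the BP_TimeManager, binds ToggleLight to its day/night state change and applies the current state.
; ToggleLight waits a random delay of up to three seconds, staggering windows, then swaps the Cube's material between Light and Dark.
; A RandomSeed is also generated at start but is not read in these graphs.
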(event `self.ReceiveBeginPlay`
  (set `self.RandomSeed` (`KismetMathLibrary.RandomFloatInRange` 0.0 1000.0))
  (bind _outactors (`GameplayStatics.GetAllActorsOfClass` "/Game/Systems/Lighting/BP_TimeManager.BP_TimeManager_C"))
  (bind _output_get (set `self.TimeManagerRef` (`|GetArrayItem` _outactors)))
  (add `/Game/Systems/Lighting/BP_TimeManager.OnDayNightStateChanged` _output_get (delegate `ToggleLight`))
  (`self.ToggleLight` (`/Game/Systems/Lighting/BP_TimeManager.CurrentIsNight` (`self.TimeManagerRef`))))

(event `ToggleLight`
  (params (CurrentIsNight :type Boolean))
  (bind _cube (`self.Cube`))
  (`KismetSystemLibrary.Delay` (`KismetMathLibrary.RandomFloatInRange` 0.0 3.0))
  (if CurrentIsNight
    (`PrimitiveComponent.SetMaterial` _cube 0 "/Game/Connor_Folder/PlaceHolder/Light.Light")
    (else
      (`PrimitiveComponent.SetMaterial` _cube 0 "/Game/Connor_Folder/PlaceHolder/Dark.Dark"))))

(event `self.ReceiveTick`
  (params (DeltaSeconds :type "Float (single-precision)")))

(fn `UserConstructionScript`)