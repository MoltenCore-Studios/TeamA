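; BP_GrindStone is an interactable sharpening station that takes input, shows WB_Sharpen and the cursor while in use.
; Alternating left/right move input builds wheel spin, which decays on Tick; forward/back flips the held item.
; A gated Tick moves a forged project to the cursor's hit point near the stone.
; A self-retriggering, speed-scaled loop capsule-traces the grind point, sending SharpenMessage with spin-based power and tag-derived side, plus sparks.
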(event `self.Exit`
  (params (Character :type "Character Object Reference"))
  (bind _returnvalue (`GameplayStatics.GetPlayerController` 0))
  (`self.DisableInput` _returnvalue)
  (set `PlayerController.bShowMouseCursor` false _returnvalue)
  (`self.CloseGate`)
  (`Widget.RemoveFromParent` (`self.WB_Sharpen`)))

(event `self.Enter`
  (params (Character :type "Character Object Reference"))
  (bind _returnvalue (`GameplayStatics.GetPlayerController` 0))
  (bind _output (`|GetArrayItem` (`self.Inventory`)))
  (set `self.Character` Character)
  (`/Engine/EditorBlueprintResources/StandardMacros.IsValid` _output
    (:`Is Valid`
      (bind _asproject (cast `Project` _output))
      (set `self.Project` _asproject))
    (:`Is Not Valid`
      _))
  (bind _returnvalue_2 (`|CreateWidget` "/Game/Connor_Folder/Sharpenning/WB_Sharpen.WB_Sharpen_C" null self))
  (bind _output_get (set `self.WB_Sharpen` _returnvalue_2))
  (`UserWidget.AddToViewport` _output_get 0)
  (`KismetSystemLibrary.PrintString` (`KismetSystemLibrary.GetDisplayName` (`|GetArrayItem` (`self.Inventory`))))
  (`self.EnableInput` _returnvalue)
  (set `PlayerController.bShowMouseCursor` true _returnvalue)
  (`self.OpenGate`))

(event `Turn`
  (bind _inventrot (`self.InventRot`))
  (bind _output (`|GetArrayItem` (`self.Inventory`)))
  (`/Engine/EditorBlueprintResources/StandardMacros.IsValid` _output
    (:`Is Valid`
      (set `self.InventRot` (`self.K2_GetActorRotation` _output))
      (bind (_direction _alpha) (`Timeline|Timeline_0` :!via `PlayFromStart`)
        (:`Update`
          (`/Engine/EditorBlueprintResources/StandardMacros.IsValid` _output
            (:`Is Valid`
              (`self.K2_SetActorRotation` _output (`KismetMathLibrary.RLerp` _inventrot (`KismetMathLibrary.MakeRotator` (.roll _inventrot) (+ (.pitch _inventrot) 180.0) (.yaw _inventrot)) _alpha true) false))))))))

(event `ContinueSpin`
  (bind _wheelrot (`self.WheelRot`))
  (set `self.WheelRot` (`SceneComponent.K2_GetComponentRotation` (`self.Spinny`)) :!label _label)
  (bind (_direction _alpha) (`Timeline|Timeline` :!via `PlayFromStart`)
    (:`Update`
      (`SceneComponent.K2_SetWorldRotation` (`self.Spinny`) (`KismetMathLibrary.RLerp` _wheelrot (`KismetMathLibrary.MakeRotator` (+ (.roll _wheelrot) (`self.SpinValue`)) (.pitch _wheelrot) (.yaw _wheelrot)) _alpha true) false false))
    (:`Finished`
      (if (> (`self.SpinValue`) 0.0)
        (`self.ContinueSpin`)))))

(event `EnhancedInput|/Game/Input/Actions/IA_Move`
  (params (ActionValue :type "Vector2D Structure") (ElapsedSeconds :type "Float (double-precision)") (TriggeredSeconds :type "Float (double-precision)") (InputAction :type "InputAction Object Reference" :default "/Game/Input/Actions/IA_Move.IA_Move"))
  (bind (_x _y) (`KismetMathLibrary.BreakVector2D` ActionValue))
  (:`Triggered`
    (if (or (and (< _x 0.0) (`self.A`)) (and (> _x 0.0) (not (`self.A`))))
      (`/Engine/EditorBlueprintResources/StandardMacros.FlipFlop`
        (:`A`
          (set `self.A` false))
        (:`B`
          (set `self.A` true)))
      (`KismetSystemLibrary.PrintString` "Hello")
      (`self.Trigger Sharpen`)
      (`KismetSystemLibrary.Delay` 0.1)
      (`self.ResetSharpen`)
      (set `self.SpinValue` (`KismetMathLibrary.FClamp` (+ (`self.SpinValue`) 4.0) 0.0 170.0))
      (goto _label)))
  (:`Started`
    (`/Engine/EditorBlueprintResources/StandardMacros.CompareFloat` _y
      (:`>`
        _)
      (:`<`
        _))
    (`/Engine/EditorBlueprintResources/StandardMacros.DoOnce` false :!label _label_2
      (:`Completed`
        (`self.Turn`)
        (`KismetSystemLibrary.Delay` 1.0)
        (goto _label_2 :!via `Reset`)))))

(event `Trigger Sharpen`
  (`/Engine/EditorBlueprintResources/StandardMacros.DoOnce` true :!label _label_3
    (:`Completed`
      (`KismetSystemLibrary.Delay` (`KismetMathLibrary.FClamp` (/ 40.0 (`self.SpinValue`)) 0.0 2.0))
      (if (> (`self.SpinValue`) 0.0)
        (`self.LineTraceGrind`)
        (`self.ResetSharpen`)
        (`self.Trigger Sharpen`)
        (`KismetSystemLibrary.RetriggerableDelay` 2.3)
        (`ActorComponent.Deactivate` (`self.Sparks`))
        (else
          (`self.ResetSharpen`))))))

(event `ResetSharpen`
  (goto _label_3 :!via `Reset`))

(event `self.ReceiveTick`
  (params (DeltaSeconds :type "Float (single-precision)"))
  (bind _project (`self.Project`))
  (bind (_hitresult _returnvalue) (`PlayerController.GetHitResultUnderCursorByChannel` (`GameplayStatics.GetPlayerController` 0) "TraceTypeQuery1" true))
  (bind _output (`|GetArrayItem` (`self.Inventory`)))
  (bind _interactionvolume (`Pickup.InteractionVolume` _output))
  (`/Engine/EditorBlueprintResources/StandardMacros.Gate` true :!label _label_4
    (:`Exit`
      (`self.Lower`)
      (`/Engine/EditorBlueprintResources/StandardMacros.IsValid` _project
        (:`Is Valid`
          (if (`Project.bIsForged` _project)
            (`/Engine/EditorBlueprintResources/StandardMacros.IsValid` _output
              (:`Is Valid`
                (if _returnvalue
                  (if (not (> (`KismetMathLibrary.Vector_Distance` (`.Location` (`GameplayStatics.BreakHitResult` _hitresult)) (`SceneComponent.K2_GetComponentLocation` (`self.Arrow`))) 400.0))
                    (`SceneComponent.K2_SetWorldLocation` _interactionvolume (`.Location` (`GameplayStatics.BreakHitResult` _hitresult)) false false)
                    (`/Engine/EditorBlueprintResources/StandardMacros.DoOnce` false :!label _label_5
                      (:`Completed`
                        (`SceneComponent.K2_SetWorldRotation` _interactionvolume (struct :`Pitch` -30.0) false false)))))))))))))

(event `OpenGate`
  (goto _label_4 :!via `Open`))

(event `CloseGate`
  (bind _output (`|GetArrayItem` (`self.Inventory`)))
  (bind _interactionvolume (`Pickup.InteractionVolume` _output))
  (`|ExecutionSequence`
    (:`then_0`
      (goto _label_4 :!via `Close`))
    (:`then_1`
      (`KismetSystemLibrary.Delay` 0.01)
      (`/Engine/EditorBlueprintResources/StandardMacros.IsValid` _output
        (:`Is Valid`
          (`SceneComponent.K2_SetWorldLocation` _interactionvolume (`SceneComponent.K2_GetComponentLocation` (`self.Item`)) false false)
          (`SceneComponent.K2_SetWorldRotation` :`self` _interactionvolume)
          (goto _label_5 :!via `Reset`))))))

(event `Lower`
  (set `self.SpinValue` (`KismetMathLibrary.FClamp` (- (`self.SpinValue`) 0.3) 0.0 170.0)))

(fn `LineTraceGrind`
  (locals (`Objects to look for` :type "Array of EObjectTypeQuery Enum") (Tags :type "Array of Name") (Index :type Integer))
  (bind _returnvalue (`SceneComponent.K2_GetComponentLocation` (`self.GrindPoint`)))
  (bind _outhit (`KismetSystemLibrary.CapsuleTraceSingleForObjects` :`Start` _returnvalue :`End` _returnvalue :`Radius` 5.0 :`HalfHeight` 30.0 :`ObjectTypes` (`local.Objects to look for`) :`DrawTime` 0.15))
  (bind (_bblockinghit _binitialoverlap _time _distance _location _impactpoint _normal _impactnormal _physmat _hitactor _hitcomponent) (`GameplayStatics.BreakHitResult` _outhit))
  (if (or _bblockinghit _binitialoverlap)
    (bind _output_get (set `local.Tags` (`ActorComponent.ComponentTags` _hitcomponent)))
    (`KismetSystemLibrary.PrintString` "ImGrinding")
    (switch `name` (`|GetArrayItem` _output_get)
      (:`L`
        (set `local.Index` 1))
      (:`R`
        (set `local.Index` 0)))
    (message `/Game/Connor_Folder/Sharpenning/BPI_Sharpen.Sharpen` (`ActorComponent.GetOwner` _hitcomponent) (/ (`self.SpinValue`) 5100.0) (`local.Index`))
    (`ActorComponent.Activate` (`self.Sparks`) true)
    (else
      (`ActorComponent.Deactivate` (`self.Sparks`)))))

(fn `RotateProject`
  (params (`X?` :type Boolean) (Value :type "Float (double-precision)"))
  (bind _output (`|GetArrayItem` (`self.Inventory`)))
  (`/Engine/EditorBlueprintResources/StandardMacros.IsValid` _output
    (:`Is Valid`
      (if `X?`
        (`self.K2_AddActorWorldRotation` _output (`KismetMathLibrary.MakeRotator` 180.0 0.0 (* (* 180.0 Value) -1.0)) false false)))))

(fn `UserConstructionScript`)