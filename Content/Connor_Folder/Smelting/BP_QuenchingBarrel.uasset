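; Quenching barrel for the smelting system that turns a filled mould into a blade.
; A half-second looping timer checks two child-actor item slots, acting only while the weapon slot is empty.
; A full BP_Mold spawns a BP_Blade with its metal and mould type into the weapon slot, plays brief steam and is deleted.
; The mould slot drops out of reach until the blade is removed, with DoOnce gates guarding both steps.
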(event `self.ReceiveBeginPlay`
  (bind _asitem_slot (cast `ItemSlot` (`ChildActorComponent.ChildActor` (`self.Mould`))))
  (set `self.MouldIS` _asitem_slot)
  (bind _asitem_slot_2 (cast `ItemSlot` (`ChildActorComponent.ChildActor` (`self.Weapon`))))
  (set `self.WeaponIS` _asitem_slot_2)
  (`KismetSystemLibrary.K2_SetTimerDelegate` (delegate `Checking`) 0.5 true))

(event `Checking`
  (bind _mouldis (`self.MouldIS`))
  (if (not (`ItemSlot.bIsOccupied` (`self.WeaponIS`)))
    (`self.Reset Mould Pos`)
    (if (`ItemSlot.bIsOccupied` _mouldis)
      (`/Engine/EditorBlueprintResources/StandardMacros.DoOnce` false :!label _label
        (:`Completed`
          (bind _asbp_mold (cast `/Game/Connor_Folder/PlaceHolder/BP_Mold` (`ItemSlot.AttachedItem` _mouldis))
            (:`then`
              (if (`/Game/Connor_Folder/PlaceHolder/BP_Mold.Full` _asbp_mold)
                (`ActorComponent.Activate` (`self.NS_SteamTest`) true)
                (bind _returnvalue (`|SpawnActorFromClass` "/Game/Connor_Folder/PlaceHolder/BP_Blade.BP_Blade_C" (`self.GetTransform`) "AlwaysSpawn" "MultiplyWithRoot" null "" "" (`/Game/Connor_Folder/PlaceHolder/BP_Mold.Metal` _asbp_mold) (`/Game/Connor_Folder/PlaceHolder/BP_Mold.MouldType` _asbp_mold) null))
                (`ItemSlot.AttachItem` (`self.WeaponIS`) _returnvalue)
                (`SceneComponent.K2_SetRelativeLocation` (`self.Mould`) (0.0 0.0 -1000.0) false false)
                (`ItemSlot.DeleteItem` (`self.MouldIS`))
                (`|ExecutionSequence`
                  (:`then_0`
                    (goto _label :!via `Reset`))
                  (:`then_1`
                    (goto _label_2 :!via `Reset`))
                  (:`then_2`
                    (`KismetSystemLibrary.Delay` 1.0)
                    (`ActorComponent.Deactivate` (`self.NS_SteamTest`))))
                (else
                  (goto _label :!via `Reset`))))
            (:`CastFailed`
              (goto _label :!via `Reset`))))))))

(event `Reset Mould Pos`
  (`/Engine/EditorBlueprintResources/StandardMacros.DoOnce` false :!label _label_2
    (:`Completed`
      (`SceneComponent.K2_SetRelativeLocation` (`self.Mould`) (0.0 0.0 0.0) false false))))

(fn `UserConstructionScript`)