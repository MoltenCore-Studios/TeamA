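; Prototype enchanting station Blueprint for drawing runes with the mouse, marked OLD by its name.
; Enter and Exit toggle input mode, cursor and a draw-sampling timer, with Exit also clearing drawn points.
; IA_DrawRune sets the drawing flag, clears points, then deprojects the cursor into a visibility line trace and prints the hit component.
; Point capture is unimplemented: the timer's SampleDrawPoint event is empty.
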(event `self.Enter`
  (params (Character :type "Character Object Reference"))
  (bind _returnvalue (`GameplayStatics.GetPlayerController` 0))
  (`WidgetBlueprintLibrary.SetInputMode_GameAndUIEx` _returnvalue null "LockOnCapture" false)
  (`self.EnableInput` _returnvalue)
  (set `PlayerController.bShowMouseCursor` true _returnvalue)
  (`self.StartDrawSampling`))

(event `self.Exit`
  (params (Character :type "Character Object Reference"))
  (bind _returnvalue (`GameplayStatics.GetPlayerController` 0))
  (`WidgetBlueprintLibrary.SetInputMode_GameOnly` _returnvalue)
  (`self.DisableInput` _returnvalue)
  (set `PlayerController.bShowMouseCursor` false _returnvalue)
  (set `self.isDrawing?` false)
  (`KismetArrayLibrary.Array_Clear` (`self.DrawnPoints`))
  (`self.StopDrawSampling`))

(event `EnhancedInput|/Game/Input/Actions/IA_DrawRune`
  (params (ActionValue :type Boolean) (ElapsedSeconds :type "Float (double-precision)") (TriggeredSeconds :type "Float (double-precision)") (InputAction :type "InputAction Object Reference" :default "/Game/Input/Actions/IA_DrawRune.IA_DrawRune"))
  (bind _returnvalue (`GameplayStatics.GetPlayerController` 0))
  (bind (_locationx _locationy _returnvalue_2) (`PlayerController.GetMousePosition` _returnvalue))
  (bind (_worldposition _worlddirection) (`GameplayStatics.DeprojectScreenToWorld` _returnvalue (`KismetMathLibrary.MakeVector2D` _locationx _locationy)))
  (:`Triggered`
    (set `self.isDrawing?` true)
    (`KismetArrayLibrary.Array_Clear` (`self.DrawnPoints`))
    (if _returnvalue_2
      (bind _outhit (`KismetSystemLibrary.LineTraceSingle` :`Start` _worldposition :`End` (+ _worldposition (* _worlddirection 5000.0)) :`TraceChannel` "TraceTypeQuery1" :`DrawDebugType` "ForDuration" :`bIgnoreSelf` false :`DrawTime` 1.0))
      (`KismetSystemLibrary.PrintString` (`KismetSystemLibrary.GetDisplayName` (`.HitComponent` (`GameplayStatics.BreakHitResult` _outhit))))))
  (:`Canceled`
    (set `self.isDrawing?` false :!label _label))
  (:`Completed`
    (goto _label)))

(event `StartDrawSampling`
  (bind _returnvalue (`KismetSystemLibrary.K2_SetTimerDelegate` (delegate `SampleDrawPoint`)))
  (set `self.DrawTimerHandle` _returnvalue))

(event `SampleDrawPoint`)

(event `StopDrawSampling`
  (`KismetSystemLibrary.K2_ClearAndInvalidateTimerHandle` (`self.DrawTimerHandle`)))

(fn `UserConstructionScript`)