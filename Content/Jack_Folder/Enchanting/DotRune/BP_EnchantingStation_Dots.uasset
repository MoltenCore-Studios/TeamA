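; BP_EnchantingStation_Dots is an enchanting station actor that lays out a grid of dot meshes, apparently for rune patterns.
; On BeginPlay it spawns a movable static mesh component per point from row count, points per row and spacing settings, offsetting odd rows by half a spacing.
; Enter and Exit events toggle actor input, mouse cursor and game/UI input mode.
; No dot selection or rune logic is implemented here.
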(event `self.ReceiveBeginPlay`
  (bind (_returnvalue_x _returnvalue_y _returnvalue_z) (`KismetMathLibrary.BreakVector` (`self.K2_GetActorLocation`)))
  (`parent.ReceiveBeginPlay`)
  ; Get the point and row index's
  (for _index (range (`self.RowCount`))
    (set `self.RowIndex` _index)
    (for _index_2 (range (`self.PointsPerRow`))
      (set `self.PointIndex` _index_2)
      ; Stagger every other row
      (if (== (mod (`self.RowIndex`) 2) 0)
        (bind _output_get (set `self.isEvenRow?` true))
        (else
          (set `self.isEvenRow?` false)))
      (set `self.BaseX` (* (`self.PointIndex`) (`self.PointSpacing`)))
      (set `self.StaggerOffset` (`KismetMathLibrary.SelectFloat` 0.0 (* (`self.PointSpacing`) 0.5) _output_get))
      (set `self.FinalX` (+ (`self.BaseX`) (`self.StaggerOffset`)))
      (set `self.FinalY` (* (`self.RowIndex`) (`self.RowSpacing`)))
      (set `self.PointLocation` (`KismetMathLibrary.MakeVector` (`self.FinalX`) (`self.FinalY`) _returnvalue_z))
      ; Add the static mesh for the point and set its location
      (bind _returnvalue (`AddComponent|NODE_AddStaticMeshComponent-2`))
      (bind _output_get_2 (set `self.PointMeshComponent` _returnvalue))
      (`StaticMeshComponent.SetStaticMesh` _output_get_2 (`self.PointMesh`))
      (`SceneComponent.SetMobility` (`self.PointMeshComponent`) "Movable")
      (`SceneComponent.K2_SetRelativeLocation` (`self.PointMeshComponent`) (`self.PointLocation`) false false))))

(event `self.Enter`
  (params (Character :type "Character Object Reference"))
  (bind _returnvalue (`GameplayStatics.GetPlayerController` 0))
  (`WidgetBlueprintLibrary.SetInputMode_GameAndUIEx` _returnvalue null "LockOnCapture" false)
  (`self.EnableInput` _returnvalue)
  (set `PlayerController.bShowMouseCursor` true _returnvalue))

(event `self.Exit`
  (params (Character :type "Character Object Reference"))
  (bind _returnvalue (`GameplayStatics.GetPlayerController` 0))
  (`WidgetBlueprintLibrary.SetInputMode_GameOnly` _returnvalue)
  (`self.DisableInput` _returnvalue)
  (set `PlayerController.bShowMouseCursor` false _returnvalue))

(fn `UserConstructionScript`
  (`parent.UserConstructionScript`))