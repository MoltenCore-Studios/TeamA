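; An enchanting station actor that opens a rune-drawing UI for the player.
; Enter switches player 0 to Game and UI input with a visible cursor, enables input on the station, then creates and shows the WBP_DrawRuneAttempt4 widget.
; Exit restores game-only input, hides the cursor, disables the station's input and removes the widget.
; BeginPlay, overlap, Tick and construction only call the parent.
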(event `self.ReceiveBeginPlay`
  (`parent.ReceiveBeginPlay`))

(event `self.ReceiveActorBeginOverlap`
  (params (OtherActor :type "Actor Object Reference"))
  (`parent.ReceiveActorBeginOverlap` OtherActor))

(event `self.ReceiveTick`
  (params (DeltaSeconds :type "Float (single-precision)"))
  (`parent.ReceiveTick` DeltaSeconds))

(event `self.Enter`
  (params (Character :type "Character Object Reference"))
  (bind _returnvalue (`GameplayStatics.GetPlayerController` 0))
  (`WidgetBlueprintLibrary.SetInputMode_GameAndUIEx` _returnvalue null "LockOnCapture" false)
  (`self.EnableInput` _returnvalue)
  (set `PlayerController.bShowMouseCursor` true _returnvalue)
  (bind _returnvalue_2 (`|CreateWidget` "/Game/Jack_Folder/Enchanting/DrawRune/UI/Attempt4/WBP_DrawRuneAttempt4.WBP_DrawRuneAttempt4_C" _returnvalue))
  (`UserWidget.AddToViewport` _returnvalue_2 0))

(event `self.Exit`
  (params (Character :type "Character Object Reference"))
  (bind _returnvalue (`GameplayStatics.GetPlayerController` 0))
  (`WidgetBlueprintLibrary.SetInputMode_GameOnly` _returnvalue)
  (`self.DisableInput` _returnvalue)
  (set `PlayerController.bShowMouseCursor` false _returnvalue)
  (`Widget.RemoveFromParent` (stale `self.Enter` _returnvalue_2)))

(fn `UserConstructionScript`
  (`parent.UserConstructionScript`))