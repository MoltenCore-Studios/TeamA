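; Test Blueprint that applies a metal preset to the shared MPC_Metal material parameter collection on BeginPlay.
; ApplyMetalFromDataTable looks up the MetalType enum name as a row in DT_Metal and caches its fields.
; It writes colours, surface, heat and rim-light values to the collection, affecting every material that reads it.
; Boolean toggles become scalars through SelectFloat, which inverts them: true gives 0, false gives 1.
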(event `self.ReceiveBeginPlay`
  (`self.Apply Metal From Data Table` (`self.Metal Type`)))

(fn `Apply Metal From Data Table`
  (params (`Metal Type` :type "/Game/Jack_Folder/Materials/E_Metal Enum" :default "NewEnumerator0"))
  (bind _output_get (set `self.Metal Type` `Metal Type`))
  (bind _returnvalue (`|GetDataTableRow` "/Game/Jack_Folder/Materials/DT_Metal.DT_Metal" (`|GetEnumeratorName` _output_get))
    (:`then`
      (set `self.Metal Colour` (break `/Game/Jack_Folder/Materials/STR_Metal` _returnvalue))
      (set `self.Imperfection Colour` (`.ImperfectionColour_5_9D1EFCFB4F3B46600FEB58A022E80A5D` (break `/Game/Jack_Folder/Materials/STR_Metal` _returnvalue)))
      (set `self.Rim Light Colour` (`.RimLightColour_7_BEE2B0E84C22DD20B7513A87AEF692B5` (break `/Game/Jack_Folder/Materials/STR_Metal` _returnvalue)))
      (set `self.Metallic` (`.Metallic_10_49F26A984FD32E55E6ED68B769ABAC2F` (break `/Game/Jack_Folder/Materials/STR_Metal` _returnvalue)))
      (set `self.Roughness` (`.Roughness_12_16436D234C643DCFD4B48D804749F2E5` (break `/Game/Jack_Folder/Materials/STR_Metal` _returnvalue)))
      (set `self.Imperfection Tiling` (`.ImperfectionTiling_14_B258F0A244B52043096AEAA05A264326` (break `/Game/Jack_Folder/Materials/STR_Metal` _returnvalue)))
      (set `self.Imperfection Strength` (`.ImperfectionStrength_16_3B78B8CC4518CE560BC448A047BAA381` (break `/Game/Jack_Folder/Materials/STR_Metal` _returnvalue)))
      (set `self.Heat Intensity` (`.HeatIntensity_18_6B99AFD048FBD09D45FDC597277360F2` (break `/Game/Jack_Folder/Materials/STR_Metal` _returnvalue)))
      (set `self.Rim Light Intensity` (`.RimLightIntensity_20_95C1A8524C2DACFB09DEBFA080A0F605` (break `/Game/Jack_Folder/Materials/STR_Metal` _returnvalue)))
      (set `self.Add Imperfection Colour` (`.AddImperfectionColour_26_41D203834891F5A3735BF4B032480723` (break `/Game/Jack_Folder/Materials/STR_Metal` _returnvalue)))
      (set `self.Enable Colour Mask` (`.EnableColourMask_25_DCC36C374D19BE10D9C294904ED76FBA` (break `/Game/Jack_Folder/Materials/STR_Metal` _returnvalue)))
      (set `self.Enable Heat` (`.EnableHeat_28_5CFEA6A74A1907DD891D0EBAD9EADD9A` (break `/Game/Jack_Folder/Materials/STR_Metal` _returnvalue)))
      (set `self.Enable Rim Light` (`.EnableRimLight_30_4361BDA244608623EA9E6AA5BF0B0380` (break `/Game/Jack_Folder/Materials/STR_Metal` _returnvalue)))
      (`KismetMaterialLibrary.SetVectorParameterValue` "/Game/Jack_Folder/Materials/MPC_Metal.MPC_Metal" "Metal Colour" (`self.Metal Colour`))
      (`KismetMaterialLibrary.SetVectorParameterValue` "/Game/Jack_Folder/Materials/MPC_Metal.MPC_Metal" "Imperfection Colour" (`self.Imperfection Colour`))
      (`KismetMaterialLibrary.SetVectorParameterValue` "/Game/Jack_Folder/Materials/MPC_Metal.MPC_Metal" "Rim Light Colour" (`self.Rim Light Colour`))
      (`KismetMaterialLibrary.SetScalarParameterValue` "/Game/Jack_Folder/Materials/MPC_Metal.MPC_Metal" "Metalic" (`self.Metallic`))
      (`KismetMaterialLibrary.SetScalarParameterValue` "/Game/Jack_Folder/Materials/MPC_Metal.MPC_Metal" "Roughness" (`self.Roughness`))
      (`KismetMaterialLibrary.SetScalarParameterValue` "/Game/Jack_Folder/Materials/MPC_Metal.MPC_Metal" "Imperfection Tiling" (`self.Imperfection Tiling`))
      (`KismetMaterialLibrary.SetScalarParameterValue` "/Game/Jack_Folder/Materials/MPC_Metal.MPC_Metal" "Imperfection Strength" (`self.Imperfection Strength`))
      (`KismetMaterialLibrary.SetScalarParameterValue` "/Game/Jack_Folder/Materials/MPC_Metal.MPC_Metal" "Heat intensity" (`self.Heat Intensity`))
      (`KismetMaterialLibrary.SetScalarParameterValue` "/Game/Jack_Folder/Materials/MPC_Metal.MPC_Metal" "Rim Light Intensity" (`self.Rim Light Intensity`))
      (`KismetMaterialLibrary.SetScalarParameterValue` "/Game/Jack_Folder/Materials/MPC_Metal.MPC_Metal" "Add Imperfection Colour" (`KismetMathLibrary.SelectFloat` 0.0 1.0 (`self.Add Imperfection Colour`)))
      (`KismetMaterialLibrary.SetScalarParameterValue` "/Game/Jack_Folder/Materials/MPC_Metal.MPC_Metal" "Enable Colour Mask" (`KismetMathLibrary.SelectFloat` 0.0 1.0 (`self.Enable Colour Mask`)))
      (`KismetMaterialLibrary.SetScalarParameterValue` "/Game/Jack_Folder/Materials/MPC_Metal.MPC_Metal" "Enable Heat?" (`KismetMathLibrary.SelectFloat` 0.0 1.0 (`self.Enable Heat`)))
      (`KismetMaterialLibrary.SetScalarParameterValue` "/Game/Jack_Folder/Materials/MPC_Metal.MPC_Metal" "Enable Rim Light?" (`KismetMathLibrary.SelectFloat` 0.0 1.0 (`self.Enable Rim Light`))))))

(fn `UserConstructionScript`)