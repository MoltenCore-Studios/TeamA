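; Smelting station minigame where the player heats crucible ore and pours it into a mould.
; Enter opens the UI and derives target temperature from the highest melting point, with averaged error margin.
; Holding Space raises heating power, release lets it decay, and looping timers update temperature and accumulate in-range time.
; After five in-range seconds, Pickup consumes the mould's ingot cost, fills it with the first ore's metal and animates the pour.
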(event `self.Enter`
  (params (Character :type "Character Object Reference"))
  (bind _smeltingui (`self.SmeltingUi`))
  (set `self.Character` Character)
  (`self.EnableInput` (`GameplayStatics.GetPlayerController` 0))
  (set `self.HowMuchOre` 0.0)
  (set `self.Target Temperature` 0.0)
  (`KismetArrayLibrary.Array_Clear` (`self.Ore`))
  (for _array_element (`BoxSlot.ContainedItems` (`self.As Box Slot`))
    (bind _asbp_ore_1 (cast `/Game/Jack_Folder/Smelting/BP_Ore1` _array_element))
    (`KismetArrayLibrary.Array_Add` (`self.Ore`) _asbp_ore_1)
    (bind (_metal_info_metalname _metal_info_descriptions _metal_info_metalmesh _metal_info_ingotvalue _metal_info_metalmaterial _metal_info_hitsneeded _metal_info_meltingpoint) (break `/Game/Connor_Folder/NoticeBoard/MetalType_Struct` (`/Game/Jack_Folder/Smelting/BP_Ore1.Metal Info` _asbp_ore_1)))
    (`self.Highest temp` _metal_info_meltingpoint)
    (`/Engine/EditorBlueprintResources/StandardMacros.IncrementFloat` (`self.HowMuchOre`)))
  (`self.SetMarginOfError`)
  (`self.Open`)
  (bind _returnvalue (`|CreateWidget` "/Game/Connor_Folder/Smelting/SmeltingUI.SmeltingUI_C" null self))
  (bind _output_get (set `self.SmeltingUi` _returnvalue))
  (set `/Game/Connor_Folder/Smelting/TempGague.SmeltingStation` self (`/Game/Connor_Folder/Smelting/SmeltingUI.TempGague` _output_get))
  (for _array_element_2 (`self.Ore`)
    (bind _metal_info_metalname_2 (break `/Game/Connor_Folder/NoticeBoard/MetalType_Struct` (`/Game/Jack_Folder/Smelting/BP_Ore1.Metal Info` _array_element_2)))
    (`/Game/Connor_Folder/Smelting/SmeltingUI.METALSIN` _smeltingui _metal_info_metalname_2))
  (`UserWidget.AddToViewport` _smeltingui 0)
  (set `PlayerController.bShowMouseCursor` true (`GameplayStatics.GetPlayerController` 0)))

(event `self.Exit`
  (params (Character :type "Character Object Reference"))
  (bind _smeltingui (`self.SmeltingUi`))
  (set `self.Character` null)
  (`self.DisableInput` (`GameplayStatics.GetPlayerController` 0))
  (`self.Close`)
  (`/Engine/EditorBlueprintResources/StandardMacros.IsValid` _smeltingui
    (:`Is Valid`
      (`Widget.RemoveFromParent` _smeltingui)
      (set `PlayerController.bShowMouseCursor` false (`GameplayStatics.GetPlayerController` 0)))))

(event `self.ReceiveBeginPlay`
  (bind _asbox_slot (cast `BoxSlot` (`ChildActorComponent.ChildActor` (`self.CrucibleContainer`))))
  (set `self.As Box Slot` _asbox_slot)
  (bind _asitem_slot (cast `ItemSlot` (`ChildActorComponent.ChildActor` (`self.MouldSpot`))))
  (set `self.As Item Slot` _asitem_slot)
  (`KismetSystemLibrary.K2_SetTimerDelegate` (delegate `LowerPower`) 0.1 true true)
  (`KismetSystemLibrary.K2_SetTimerDelegate` (delegate `CrucibleStuff`) 0.01 true true)
  (`KismetSystemLibrary.K2_SetTimerDelegate` (delegate `Check Crucible Temperature`) 0.1 true true))

(event `LowerPower`
  (`/Engine/EditorBlueprintResources/StandardMacros.Gate` true :!label _label
    (:`Exit`
      (set `self.HeatingPower` (`KismetMathLibrary.FClamp` (- (`self.HeatingPower`) 1.0) -15.0 10.0)))))

(event `OpenLowerPower`
  (params (Return :type Boolean))
  (if Return
    (goto _label :!via `Open`)
    (else
      (goto _label :!via `Close`))))

(event `self.ReceiveTick`
  (params (DeltaSeconds :type "Float (single-precision)"))
  (`self.Print Metal Info`))

(event `CrucibleStuff`
  (`self.Heat Crucible`))

(event `Check Crucible Temperature`
  (bind _marginoferror_per_side_ (`self.MarginOfError(per side)`))
  (bind _target_temperature (`self.Target Temperature`))
  (if (`KismetMathLibrary.InRange_FloatFloat` (`self.CrucibleTemperature`) (- _target_temperature _marginoferror_per_side_) (+ _target_temperature _marginoferror_per_side_))
    (bind _output_get (set `self.TimeInSmelter` (`KismetMathLibrary.FClamp` (+ (`self.TimeInSmelter`) 0.1) 0.0 5.0)))
    (`KismetSystemLibrary.PrintString` (`KismetStringLibrary.Conv_DoubleToString` _output_get))
    (if (>= (`self.TimeInSmelter`) 5.0)
      _)))

(event `EnhancedInput|/Game/Input/Actions/IA_Pickup`
  (params (ActionValue :type Boolean) (ElapsedSeconds :type "Float (double-precision)") (TriggeredSeconds :type "Float (double-precision)") (InputAction :type "InputAction Object Reference" :default "/Game/Input/Actions/IA_Pickup.IA_Pickup"))
  (bind _returnvalue (`GameplayStatics.GetPlayerController` 0))
  (bind _smeltingui (`self.SmeltingUi`))
  (bind _as_item_slot (`self.As Item Slot`))
  (bind _metalpour1 (`self.METALPOUR1`))
  (bind (_weaponstruct_weaponname _weaponstruct_descriptions _weaponstruct_ingotcost) (break `/Game/Connor_Folder/NoticeBoard/WeaponType_Struct` (`/Game/Connor_Folder/PlaceHolder/BP_Mold.WeaponStruct` (`self.As BP Mold`))))
  (bind _containeditems (`BoxSlot.ContainedItems` (`self.As Box Slot`)))
  (:`Started`
    (if (and (`ItemSlot.bIsOccupied` _as_item_slot) (== (`self.TimeInSmelter`) 5.0))
      (bind _asbp_mold (cast `/Game/Connor_Folder/PlaceHolder/BP_Mold` (`ItemSlot.AttachedItem` _as_item_slot)))
      (bind _output_get (set `self.As BP Mold` _asbp_mold))
      (if (and (not (`/Game/Connor_Folder/PlaceHolder/BP_Mold.Full` _output_get)) (>= (`self.HowMuchOre`) _weaponstruct_ingotcost))
        (`/Engine/EditorBlueprintResources/StandardMacros.DoOnce` false :!label _label_2
          (:`Completed`
            (set `self.HowMuchOre` (- (`self.HowMuchOre`) _weaponstruct_ingotcost))
            (`self.MetalNameToEnum`)
            (for _ (range (`KismetMathLibrary.FTrunc` _weaponstruct_ingotcost))
              (`self.K2_DestroyActor` (`|GetArrayItem` _containeditems))
              (`KismetArrayLibrary.Array_Remove` _containeditems)
              (`KismetArrayLibrary.Array_Remove` (`self.Ore`)))
            (set `/Game/Connor_Folder/PlaceHolder/BP_Mold.Full` true (`self.As BP Mold`))
            (`/Game/Connor_Folder/Smelting/SmeltingUI.Reset` _smeltingui)
            (for _array_element (`self.Ore`)
              (bind _metal_info_metalname (break `/Game/Connor_Folder/NoticeBoard/MetalType_Struct` (`/Game/Jack_Folder/Smelting/BP_Ore1.Metal Info` _array_element)))
              (`/Game/Connor_Folder/Smelting/SmeltingUI.METALSIN` _smeltingui _metal_info_metalname))
            (`self.DisableInput` (`self.Character`) (`GameplayStatics.GetPlayerController` 0))
            (`SceneComponent.SetVisibility` (`self.METALPOUR1`) true false)
            (`SkeletalMeshComponent.PlayAnimation` (`self.Crucible1`) "/Game/Connor_Folder/Smelting/ConnorMadeModels/Crucible_Anim_Armature_001_Armature_001Action_001.Crucible_Anim_Armature_001_Armature_001Action_001" false)
            (`SkeletalMeshComponent.PlayAnimation` _metalpour1 "/Game/Connor_Folder/Smelting/ConnorMadeModels/Turn.Turn" false)
            (`KismetSystemLibrary.Delay` 1.2)
            (`SkeletalMeshComponent.PlayAnimation` _metalpour1 "/Game/Connor_Folder/Smelting/ConnorMadeModels/Pour.Pour" false)
            (`KismetSystemLibrary.Delay` 3.0)
            (`self.EnableInput` (`self.Character`) _returnvalue)
            (`WidgetBlueprintLibrary.SetInputMode_GameOnly` _returnvalue true)
            (`SceneComponent.SetVisibility` (`self.METALPOUR1`) false false)
            (`SkeletalMeshComponent.PlayAnimation` (`self.Crucible1`) "/Game/Connor_Folder/Smelting/ConnorMadeModels/Crucibleturnup.Crucibleturnup" false)
            (`self.PourReset`))))
      (else
        (`KismetSystemLibrary.PrintString` "Metal not hot enough OR no mould")))))

(event `EnhancedInput|/Game/Input/Actions/IA_Space`
  (params (ActionValue :type Boolean) (ElapsedSeconds :type "Float (double-precision)") (TriggeredSeconds :type "Float (double-precision)") (InputAction :type "InputAction Object Reference" :default "/Game/Input/Actions/IA_Space.IA_Space"))
  ; For now changed it to held. Can be changed
  (:`Started`
    (`self.OpenLowerPower` false :!label _label_3)
    (set `self.HeatingPower` (`KismetMathLibrary.FClamp` (+ (`self.HeatingPower`) 0.05) -15.0 10.0)))
  (:`Ongoing`
    (goto _label_3))
  (:`Canceled`
    (`self.OpenLowerPower` true :!label _label_4))
  (:`Completed`
    (goto _label_4)))

(event `MetalNameToEnum`
  (bind _as_bp_mold (`self.As BP Mold`))
  (bind _metal_info_metalname (break `/Game/Connor_Folder/NoticeBoard/MetalType_Struct` (`/Game/Jack_Folder/Smelting/BP_Ore1.Metal Info` (`|GetArrayItem` (`self.Ore`)))))
  (switch `string` _metal_info_metalname
    (:`Iron`
      (set `/Game/Connor_Folder/PlaceHolder/BP_Mold.Metal` "NewEnumerator0" _as_bp_mold))
    (:`Gold`
      (set `/Game/Connor_Folder/PlaceHolder/BP_Mold.Metal` "NewEnumerator1" _as_bp_mold))
    (:`Tungsten`
      (set `/Game/Connor_Folder/PlaceHolder/BP_Mold.Metal` "NewEnumerator2" _as_bp_mold))
    (:`Copper`
      (set `/Game/Connor_Folder/PlaceHolder/BP_Mold.Metal` "NewEnumerator3" _as_bp_mold))))

(event `PourReset`
  (set `self.TimeInSmelter` 0.0)
  (goto _label_2 :!via `Reset`))

(event `Heat Crucible`
  (set `self.CrucibleTemperature` (`KismetMathLibrary.FClamp` (+ (`self.CrucibleTemperature`) (`self.HeatingPower`)) 0.0 4000.0))
  (if (== (`self.CrucibleTemperature`) 0.0)
    (set `self.HeatingPower` 0.0)))

(event `Cool Crucible`
  (set `self.CrucibleTemperature` (`KismetMathLibrary.FClamp` (- (`self.CrucibleTemperature`) 1.0) 0.0 4000.0)))

(event `Print Metal Info`
  (`/Engine/EditorBlueprintResources/StandardMacros.Gate` true :!label _label_5
    (:`Exit`
      (`KismetSystemLibrary.PrintString` (`KismetStringLibrary.Concat_StrStr` "Metal Name:  " (`self.Metal Name`)) true true (struct :`R` 1.0 :`G` 0.520996 :`B` 0.001821 :`A` 1.0) 0.0)
      (`KismetSystemLibrary.PrintString` (`KismetStringLibrary.Concat_StrStr` "Target Temperature:  " (`KismetStringLibrary.Conv_DoubleToString` (`self.Target Temperature`))) true true (struct :`R` 1.0 :`G` 0.522747 :`B` 0.001823 :`A` 1.0) 0.0))))

(event `Open`
  (goto _label_5 :!via `Open`))

(event `Close`
  (goto _label_5 :!via `Close`))

(fn `Highest temp`
  (params (MeltingPoint :type "Float (double-precision)"))
  (if (> MeltingPoint (`self.Target Temperature`))
    (set `self.Target Temperature` MeltingPoint)))

(fn `SetMarginOfError`
  (bind _ore (`self.Ore`))
  (set `self.MarginOfError(per side)` 0.0)
  (for _array_element _ore
    (bind (_metal_info_metalname _metal_info_descriptions _metal_info_metalmesh _metal_info_ingotvalue _metal_info_metalmaterial _metal_info_hitsneeded _metal_info_meltingpoint _metal_info_marginoferrorperside) (break `/Game/Connor_Folder/NoticeBoard/MetalType_Struct` (`/Game/Jack_Folder/Smelting/BP_Ore1.Metal Info` _array_element)))
    (set `self.MarginOfError(per side)` (+ (`self.MarginOfError(per side)`) _metal_info_marginoferrorperside)))
  (set `self.MarginOfError(per side)` (/ (`self.MarginOfError(per side)`) (`KismetArrayLibrary.Array_Length` _ore))))

(fn `UserConstructionScript`)