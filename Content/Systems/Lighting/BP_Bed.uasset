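; Interactable bed that lets the player sleep through the night and skip to morning.
; A trigger box shows a prompt and enables input while a Character overlaps it.
; Pressing E looks up BP_TimeManager and, during night hours only, locks movement, fades out the camera, calls SkipToMorning, then fades back in.
; An IsSleeping flag blocks re-entry; rejected presses print a message.
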(event `self.TriggerBox.OnComponentBeginOverlap`
  (params (OverlappedComponent :type "PrimitiveComponent Object Reference") (OtherActor :type "Actor Object Reference") (OtherComp :type "PrimitiveComponent Object Reference") (OtherBodyIndex :type Integer) (bFromSweep :type Boolean) (SweepResult :type "HitResult Structure (by ref)"))
  (cast `Character` OtherActor)
  (`self.EnableInput` (`GameplayStatics.GetPlayerController` 0))
  (`SceneComponent.SetVisibility` (`self.PromptText`) true false))

(event `self.TriggerBox.OnComponentEndOverlap`
  (params (OverlappedComponent :type "PrimitiveComponent Object Reference") (OtherActor :type "Actor Object Reference") (OtherComp :type "PrimitiveComponent Object Reference") (OtherBodyIndex :type Integer))
  (cast `Character` OtherActor)
  (`self.DisableInput` (`GameplayStatics.GetPlayerController` 0))
  (`SceneComponent.SetVisibility` (`self.PromptText`) false false))

(event `Key|E`
  (params (Key :type "Key Structure"))
  (bind _currenttime (`/Game/Systems/Lighting/BP_TimeManager.CurrentTime` (`self.TimeManagerRef`)))
  (:`Pressed`
    (if (`self.IsSleeping`)
      (`KismetSystemLibrary.PrintString` "You are already sleeping!")
      (else
        (bind _returnvalue (`GameplayStatics.GetActorOfClass` "/Game/Systems/Lighting/BP_TimeManager.BP_TimeManager_C"))
        (set `self.TimeManagerRef` _returnvalue)
        (if (or (> _currenttime 20.0) (< _currenttime 5.0))
          (set `self.IsSleeping` true)
          (bind _returnvalue_2 (`InputDeviceLibrary.GetPlayerControllerFromInputDevice` (struct)))
          (`Controller.SetIgnoreMoveInput` (`GameplayStatics.GetPlayerController` 0) true)
          (bind _playercameramanager (`PlayerController.PlayerCameraManager` _returnvalue_2))
          (`PlayerCameraManager.StartCameraFade` :`self` _playercameramanager :`ToAlpha` 1.0 :`Duration` 1.5 :`bShouldFadeAudio` true :`bHoldWhenFinished` true)
          (`KismetSystemLibrary.Delay` 2.0)
          (`/Game/Systems/Lighting/BP_TimeManager.SkipToMorning` (`self.TimeManagerRef`))
          (`KismetSystemLibrary.Delay` 1.0)
          (`PlayerCameraManager.StartCameraFade` :`self` _playercameramanager :`FromAlpha` 1.0 :`Duration` 1.5)
          (`InputDeviceLibrary.GetPlayerControllerFromInputDevice` (struct))
          (`Controller.SetIgnoreMoveInput` (`GameplayStatics.GetPlayerController` 0) false)
          (set `self.IsSleeping` false)
          (else
            (`KismetSystemLibrary.PrintString` "It is too early to sleep." true true (struct :`R` 1.0 :`A` 1.0))))))))

(fn `UserConstructionScript`)