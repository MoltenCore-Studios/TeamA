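; BP_TimeManager runs a day/night cycle, tracking time of day and day count while rotating the SunLight actor to match.
; Each Tick advances CurrentTime by TimeSpeed, wraps it at 24 hours with a day increment and debug print, then maps it linearly to sun pitch.
; A W_DebugHUD widget, created on BeginPlay, receives the current time and day every frame.
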(event `self.ReceiveBeginPlay`
  (bind _returnvalue (`|CreateWidget` "/Game/Systems/Lighting/W_DebugHUD.W_DebugHUD_C"))
  (bind _output_get (set `self.MyHUD` _returnvalue))
  (`UserWidget.AddToViewport` _output_get 0))

(event `self.ReceiveTick`
  (params (DeltaSeconds :type "Float (single-precision)"))
  (set `self.CurrentTime` (+ (* DeltaSeconds (`self.TimeSpeed`)) (`self.CurrentTime`)))
  (if (>= (`self.CurrentTime`) 24.0)
    (set `self.CurrentTime` 0.0)
    (bind _result (`/Engine/EditorBlueprintResources/StandardMacros.IncrementInt` (`self.DayCount`))
      (:`  `
        (`KismetSystemLibrary.PrintString` "NEW DAY!" true true (struct :`R` 1.0 :`A` 1.0)))))
  (`self.K2_SetActorRotation` (`self.SunLight`) (`KismetMathLibrary.MakeRotator` 0.0 (* (- (`self.CurrentTime`) 6.0) 15.0)) false)
  (`/Game/Systems/Lighting/W_DebugHUD.UpdateDebugInfo` (`self.MyHUD`) (`self.CurrentTime`) (`self.DayCount`)))

(fn `UserConstructionScript`)