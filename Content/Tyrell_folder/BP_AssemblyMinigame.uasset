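; BP_AssemblyMinigame runs a timing-bar riveting minigame started from a workbench.
; It shows a WBP_TimingBar widget, scores each hit input by Red, Yellow or Green zone, then re-randomizes the zones.
; A rivet completes at a progress threshold and logs its hit count; after the last, the game ends and the workbench attaches the handle.
; A state enum gates input and lets restart reset only unfinished runs.
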(event `self.ReceiveBeginPlay`)

(event `StartMinigame()`
  (params (WorkBench :type "/Game/Blueprints/Tyrell_workstation Object Reference"))
  ; Starts Minigame which will have 4 states
  (set `self.Work Bench` WorkBench)
  (set `self.CurrentState` "NewEnumerator1")
  (bind _returnvalue (`|CreateWidget` "/Game/Tyrell_folder/WBP_TimingBar.WBP_TimingBar_C" (`GameplayStatics.GetPlayerController` 0)))
  (bind _output_get (set `self.TimingWidgetRef` _returnvalue))
  (`UserWidget.AddToViewport` _output_get 0)
  (`KismetSystemLibrary.PrintString` "add to viewport is runing")
  (`/Game/Tyrell_folder/WBP_TimingBar.RandomizeZones` (`self.TimingWidgetRef`)))

(event `BeginRivet`
  (params (Index :type Integer))
  (set `self.CurrentRivetIndex` Index)
  (set `self.CurrentProgress` 0)
  (set `self.HitsThisRivet` 0))

(event `HandleHitInput`
  (`KismetSystemLibrary.PrintString` "handlehitinput is running")
  (if (`|EnumEquality` (`self.CurrentState`) "NewEnumerator1")
    (`/Engine/EditorBlueprintResources/StandardMacros.IsValid` (`self.TimingWidgetRef`)
      (:`Is Valid`
        (bind _result (`/Game/Tyrell_folder/WBP_TimingBar.EvaluateHit` (`self.TimingWidgetRef`)))
        (switch `/Game/Tyrell_folder/EAccuracyZone` _result
          (:`NewEnumerator0`
            (set `self.Points` 1))
          (:`NewEnumerator1`
            (set `self.Points` 3))
          (:`NewEnumerator2`
            (set `self.Points` 5)))
        (set `self.CurrentProgress` (+ (`self.CurrentProgress`) (`self.Points`)))
        (set `self.HitsThisRivet` (+ (`self.HitsThisRivet`) 1))
        (if (>= (`self.CurrentProgress`) 10)
          (`KismetArrayLibrary.Array_Add` (`self.RivetHits`) (`self.HitsThisRivet`))
          (set `self.CurrentRivetIndex` (+ (`self.CurrentRivetIndex`) 1))
          (set `self.CurrentProgress` 0)
          (set `self.HitsThisRivet` 0)
          (`/Game/Tyrell_folder/WBP_TimingBar.RandomizeZones` (`self.TimingWidgetRef`))
          (if (>= (`self.CurrentRivetIndex`) (`self.TotalRivets`))
            (`self.EndMinigame`)
            (`/Game/Blueprints/Tyrell_workstation.AttachHandle` (`self.Work Bench`))
            (else
              (set `self.CurrentState` "NewEnumerator1")))
          (else
            ; if false, randomise zone, or you can get rid of this if you don't want this function
            (`/Game/Tyrell_folder/WBP_TimingBar.RandomizeZones` (`self.TimingWidgetRef`)))))
      (:`Is Not Valid`
        (`KismetSystemLibrary.PrintString` "No Widget Ref")))))

(event `EndMinigame`
  (`KismetSystemLibrary.PrintString` "Minigame is finished")
  (set `self.CurrentState` "NewEnumerator3")
  (`Widget.RemoveFromParent` (`self.TimingWidgetRef`))
  (set `self.CurrentRivetIndex` 0)
  (set `self.HitsThisRivet` 0)
  (set `self.CurrentProgress` 0))

(event `Restart_minigame`
  (if (`|EnumEquality` (`self.CurrentState`) "NewEnumerator3")
    (`KismetSystemLibrary.PrintString` "User actually finished minigame")
    (else
      (`KismetSystemLibrary.PrintString` "Minigame didn't finish completely")
      (set `self.CurrentState` "NewEnumerator0")
      (`Widget.RemoveFromParent` (`self.TimingWidgetRef`))
      (set `self.CurrentRivetIndex` 0)
      (set `self.HitsThisRivet` 0)
      (set `self.CurrentProgress` 0))))

(fn `UserConstructionScript`)